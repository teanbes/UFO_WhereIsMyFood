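; Corral actor that acts as the scoring and game-over zone, built around a Trigger component.
; Every Tick it copies the Trigger's count into CurrentScore on the Where Is My Food game mode.
; Half a second after an overlap begins, it asks the Trigger whether the game is over, with debug prints.
; If so, it shows the end screen, switches to UI-only input with a cursor and ignores player movement.
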(event OnComponentBeginOverlap(Trigger)
  (params (OverlappedComponent :type Primitive%20Component%20Object%20Reference) (OtherActor :type Actor%20Object%20Reference) (OtherComp :type Primitive%20Component%20Object%20Reference) (OtherBodyIndex :type Integer) (bFromSweep :type Boolean) (SweepResult :type Hit%20Result%20Structure%20%28by%20ref%29))
  (bind _returnvalue (Game|GetPlayerController 0))
  (bind _trigger (Variables|Default|GetTrigger))
  (bind _returnvalue_2 (Class|TriggerComponent|IsGameOver _trigger))
  (Utilities|FlowControl|Delay 0.5)
  (Development|PrintString (Utilities|GetDisplayName OtherActor))
  (if _returnvalue_2
    (bind _returnvalue_3 (UserInterface|CreateWidget "/Game/_Game/HUD/WBP_EndScreen.WBP_EndScreen_C"))
    (UserInterface|Viewport|AddtoViewport _returnvalue_3 0)
    ;[1 1 1] Ignoring player movement and setting input mode to UI
    (Input|SetInputModeUIOnly _returnvalue _returnvalue_3 "DoNotLock" true)
    (Variables|/Script/Engine.PlayerController|SetbShowMouseCursor _returnvalue true)
    (Input|SetIgnoreMoveInput _returnvalue true)
    (else
      (Development|PrintString (Utilities|String|ToString(Boolean) _returnvalue_2)))))

(event EventBeginPlay)

(event Collision|EventActorBeginOverlap
  (params (OtherActor :type Actor%20Object%20Reference)))

(event EventTick
  (params (DeltaSeconds :type Float%20%28single-precision%29))
  (bind _asbp_where_is_my_food_game_mode_base (Utilities|Casting|CastToBP_WhereIsMyFoodGameModeBase (Game|GetGameMode)))
  (Variables|/Game/_Game/GameMode/BP_WhereIsMyFoodGameModeBase.BP_WhereIsMyFoodGameModeBase_C|SetCurrentScore _asbp_where_is_my_food_game_mode_base (Class|TriggerComponent|GetAmountOfTriggers (Variables|Default|GetTrigger))))

(fn ConstructionScript)