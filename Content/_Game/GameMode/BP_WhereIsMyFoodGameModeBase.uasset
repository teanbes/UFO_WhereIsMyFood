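; Game mode for WhereIsMyFood that sets game-only input and tracks a pig-based win condition.
; Shortly after BeginPlay, it sets MaxScore to the number of BP_Pig actors, then stores and prints whether CurrentScore already equals it.
; A delayed Tick check repeats roughly every three seconds and only prints CurrentScore when it matches MaxScore.
; Nothing here changes CurrentScore or acts on a win beyond debug printing.
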(event EventBeginPlay
  (Utilities|FlowControl|Delay 0.5)
  (Input|SetInputModeGameOnly (Game|GetPlayerController 0) false)
  (bind _outactors (Actor|GetAllActorsOfClass "/Game/_Game/Blueprints/BP_Pig.BP_Pig_C"))
  (bind _output_get (Variables|Default|SetMaxScore (Utilities|Array|Length _outactors)))
  (bind _output_get_2 (Variables|Default|SetWinCondition (== (Variables|Default|GetCurrentScore) _output_get)))
  (Development|PrintString (Utilities|String|ToString(Boolean) _output_get_2) true true "(R=0.000000,G=0.660000,B=1.000000,A=1.000000)" 4.0))

(event EventTick
  (params (DeltaSeconds :type Float%20%28single-precision%29))
  (bind _currentscore (Variables|Default|GetCurrentScore))
  (Utilities|FlowControl|Delay 3.0)
  (if (== _currentscore (Variables|Default|GetMaxScore))
    (Development|PrintString (Utilities|String|ToString(Integer) _currentscore))))

(fn ConstructionScript)